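; Skeleton enemy AI pawn that chases the player on sight and plays a sword attack, apparently work in progress.
; PawnSensing sets a seen flag and calls FollowPlayer, which uses AI MoveTo toward the player character.
; On arrival it plays the attack animation once: CanAttack is cleared and never restored after the trailing delay.
; The seen flag is never cleared, and the ApplyDamage node is unconnected, so attacks deal no damage.
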(event OnSeePawn(PawnSensing)
  (params (Pawn :type Pawn%20Object%20Reference))
  (Variables|Default|SetisSeeingPlayer true)
  (CallFunction|FollowPlayer))

(event Custom|FollowPlayer
  (if (Variables|Default|GetisSeeingPlayer)
    (AI|AIMoveTo self "0, 0, 0" (Game|GetPlayerCharacter 0) 7e+01 false
      (:OnSuccess
        (if (Variables|Default|GetcanAttack)
          (Variables|Default|SetcanAttack false)
          (Components|Animation|PlayAnimation (Variables|Character|GetMesh) "/Game/UndeadPack/SkeletonEnemy/Animations/Anim_Attack_Sword_1.Anim_Attack_Sword_1" false)
          (Utilities|FlowControl|Delay 2.0))))))

(event EventBeginPlay)

(event Collision|EventActorBeginOverlap
  (params (OtherActor :type Actor%20Object%20Reference)))

(fn ConstructionScript)
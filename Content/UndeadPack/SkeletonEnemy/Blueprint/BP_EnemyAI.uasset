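; BP_EnemyAI is a skeleton enemy that chases and attacks the player.
; Pawn sensing latches a seen flag and starts AI MoveTo, playing a sword animation on arrival, gated by a two-second cooldown.
; A box overlap deals fixed damage independently of the attack state.
; Incoming damage reduces clamped health; death only sets a flag, as the destroy logic is unconnected.
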(event OnSeePawn(PawnSensing)
  (params (Pawn :type Pawn%20Object%20Reference))
  (Variables|Default|SetisSeeingPlayer true)
  (CallFunction|FollowPlayer))

(event OnComponentBeginOverlap(Box)
  (params (OverlappedComponent :type Primitive%20Component%20Object%20Reference) (OtherActor :type Actor%20Object%20Reference) (OtherComp :type Primitive%20Component%20Object%20Reference) (OtherBodyIndex :type Integer) (bFromSweep :type Boolean) (SweepResult :type Hit%20Result%20Structure%20%28by%20ref%29))
  (Game|Damage|ApplyDamage OtherActor 2e+01 0 self))

(event Custom|FollowPlayer
  (if (Variables|Default|GetisSeeingPlayer)
    (AI|AIMoveTo self "0, 0, 0" (Game|GetPlayerCharacter 0) 7e+01 false
      (:OnSuccess
        (if (Variables|Default|GetcanAttack)
          (Variables|Default|SetcanAttack false)
          (Components|Animation|PlayAnimation (Variables|Character|GetMesh) "/Game/UndeadPack/SkeletonEnemy/Animations/Anim_Attack_Sword_1.Anim_Attack_Sword_1" false)
          (Utilities|FlowControl|Delay 2.0)
          (Variables|Default|SetcanAttack true))))))

(event Custom|Die
  (Variables|Default|SetisDead true))

(event EventBeginPlay)

(event Game|Damage|EventAnyDamage
  (params (Damage :type Float%20%28single-precision%29) (DamageType :type Damage%20Type%20Object%20Reference) (InstigatedBy :type Controller%20Object%20Reference) (DamageCauser :type Actor%20Object%20Reference))
  (bind _output_get (Variables|Default|Sethealth (Math|Float|Clamp(Float) (- (Variables|Default|Gethealth) Damage) 0.0 (Variables|Default|Getmax%20health))))
  (if (<= _output_get 0.0)
    (CallFunction|Die)))

(event Collision|EventActorBeginOverlap
  (params (OtherActor :type Actor%20Object%20Reference)))

(fn ConstructionScript)